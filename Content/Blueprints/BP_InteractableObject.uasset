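; Interactable object actor that shows its type and material options once it has been touched for a set delay.
; Touch events, fired from outside, send the type to a linked printable wall mount and start the Custom HUD crosshair countdown.
; A retriggerable delay flags completion if still touched, and a Tick-driven gate then passes text, actor and materials to the HUD.
; The construction script applies the configured mesh and material.
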(event `self.ReceiveTick`
  (params (DeltaSeconds :type "Float (single-precision)"))
  ;[1 1 1] Checking on Notification To HUD
  (`/Engine/EditorBlueprintResources/StandardMacros.Gate` true :!label _label
    (:`Exit`
      (if (`self.isTimerFinished`)
        (`self.NotifyHUDToPrintText`)
        (`KismetSystemLibrary.PrintString` "COMPLETE!!!!!!!!!!!!")
        (set `self.isTimerFinished` false)
        (else
          (`KismetSystemLibrary.Delay` 1.0)
          (`KismetSystemLibrary.PrintString` "UI CANCELED"))))))

(event `self.ReceiveBeginPlay`
  ;[1 1 1] Get CustomHUD reference
  (bind _ascustom_hud (cast `/Game/Menus/Custom_HUD` (`PlayerController.GetHUD` (`GameplayStatics.GetPlayerController` 0))))
  (set `self.m_CustomHUD` _ascustom_hud))

(event `ObjectUnTouched_Event`
  ;[1 1 1] Object Untouched
  (`KismetSystemLibrary.PrintString` "WOW UNTOUCHED")
  (`/Game/Menus/Custom_HUD.OnObjectUntouched_HUD` (`self.m_CustomHUD`))
  (set `self.m_IsTouching` false)
  (set `self.isTimerFinished` false)
  (goto _label :!via `Close`))

(event `ObjectTouched_Event`
  ;[1 1 1] On object TOuched
  (`KismetSystemLibrary.PrintString` "WOW TOuched")
  (bind _output_get (set `self.m_TextToPrint` (`KismetTextLibrary.Conv_StringToText` (`self.m_ObjectType`))))
  (bind _asbp_printable_wall_mount (cast `/Game/FirstPersonBP/Blueprints/BP_PrintableWallMount` (`self.m_WallMount`)))
  (`/Game/FirstPersonBP/Blueprints/BP_PrintableWallMount.PrintObjectInfo_Event` _asbp_printable_wall_mount _output_get)
  (set `self.m_IsTouching` true)
  (`/Game/Menus/Custom_HUD.OnCustomHUDNotifyCrosshair` (`self.m_CustomHUD`) (`self.m_DelayInSecond`))
  (`KismetSystemLibrary.PrintString` "WAITING............")
  (`self.StartLockTimer`)
  (goto _label :!via `Open`))

(event `StartLockTimer`
  ;[1 1 1] Event Start Info Timer
  (`KismetSystemLibrary.RetriggerableDelay` (`KismetMathLibrary.Conv_IntToDouble` (`self.m_DelayInSecond`)))
  (if (`self.m_IsTouching`)
    (set `self.isTimerFinished` true)
    (else
      (set `self.isTimerFinished` false))))

(fn `ExecuteCalling`)

(fn `InitCustomMaterialUI`
  (for _ (`self.m_MaterialCollection`)
    _))

(fn `NotifyHUDToPrintText`
  (`/Game/Menus/Custom_HUD.OnObjectTouched_HUD` (`self.m_CustomHUD`) (`self.m_TextToPrint`) self (`self.m_MaterialCollection`)))

(fn `UserConstructionScript`
  (bind _placeholderobject (`self.PlaceholderObject`))
  (`StaticMeshComponent.SetStaticMesh` _placeholderobject (`self.m_Object`))
  (`PrimitiveComponent.SetMaterial` _placeholderobject 0 (`self.m_ObjectMaterial`)))